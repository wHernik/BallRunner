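; BP_Cannon is an automatic cannon actor that repeatedly fires projectiles from the moment play begins.
; After each FireRate delay, it spawns a BP_Projectile at the ProjectileSpawn component's location and rotation, scaled by ProjectileScale.
; A timeline then animates barrel recoil along the relative Y axis, and its Cannon Fired output loops back to the delay for the next shot.
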(event EventBeginPlay
  (Utilities|FlowControl|Delay (Variables|CannonProperties|GetFire%20Rate) :!label _label)
  (CallFunction|SpawnProjectile)
  (bind _cannon_recoil (Timeline|Cannon%20Fire%20Movement PlayFromStart)
    (:Update
      (CallFunction|BarrelMovement _cannon_recoil))
    (:Cannon%20Fired
      (goto _label))))

(fn ConstructionScript)

(fn SpawnProjectile
  (bind _projectile_spawn (Variables|Default|GetProjectile%20Spawn))
  (Game|SpawnActorfromClass "/Game/Blueprints/Actors/Projectile/BP_Projectile.BP_Projectile_C" (Math|Transform|MakeTransform (Transformation|GetWorldLocation _projectile_spawn) (Transformation|GetWorldRotation _projectile_spawn) (Math|Conversions|ToVector(Float) (Variables|CannonProperties|GetProjectile%20Scale))) "Undefined" 0 0))

(fn BarrelMovement
  (params (BArrel_Y_Location :type Float%20%28single-precision%29))
  (Transformation|SetRelativeLocation (Variables|Default|GetCannon_Barrel) (Math|Vector|MakeVector 0.0 BArrel_Y_Location 0.0) false false))