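; BP_Spike is a hazard actor whose cone spike moves vertically on a repeating cycle and damages the player.
; From BeginPlay it waits for Duration, then plays the Spike_Movement timeline, whose UpDown track drives the cone's relative Z through SpikeMove.
; The timeline's Moved output loops back to the delay to repeat the cycle.
; Any actor overlap that passes IsPlayer applies damage to player pawn 0.
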(event EventBeginPlay
  (Utilities|FlowControl|Delay (Variables|Default|GetDuration) :!label _label)
  (bind _up_down (Timeline|Spike_Movement PlayFromStart)
    (:Update
      (CallFunction|SpikeMove _up_down))
    (:Moved
      (goto _label))))

(event Collision|EventActorBeginOverlap
  (params (OtherActor :type Actor%20Object%20Reference))
  (Utilities|IsPlayer OtherActor
    (:Is%20Player
      (Game|Damage|ApplyDamage (Game|Player|GetPlayerPawn 0) 1.0 0 0))))

(fn ConstructionScript)

(fn SpikeMove
  (params (Spike%20Z%20Location :type Float%20%28single-precision%29))
  (Transformation|SetRelativeLocation (Variables|Default|GetCone) (Math|Vector|MakeVector 0.0 0.0 Spike%20Z%20Location) false false))