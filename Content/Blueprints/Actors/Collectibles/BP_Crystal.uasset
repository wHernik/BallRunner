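; BP_Crystal is a collectible crystal that plays a pickup animation when the player overlaps it, then destroys itself.
; On overlap it caches its location, scale and light intensity, plus the player pawn's position.
; The TL_BlendAlpha timeline drives separate lerps that move it to that position, shrink it to zero and fade its PointLight.
; The target is captured once, so the crystal does not follow a moving pawn.
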(event Collision|EventActorBeginOverlap
  (params (OtherActor :type Actor%20Object%20Reference))
  (Utilities|IsPlayer OtherActor
    (:Is%20Player
      (CallFunction|SetVariables)
      (bind (_direction _crystal_location _crystal_scale _crystal_light) (Timeline|TL_BlendAlpha Play)
        (:Update
          (CallFunction|MoveCrystaltoPawn _crystal_location)
          (CallFunction|CrystalScale _crystal_scale)
          (CallFunction|CrystalLight _crystal_light))
        (:Finished
          (Actor|DestroyActor))))))

(fn ConstructionScript)

(fn MoveCrystaltoPawn
  (params (Alpha :type Float%20%28single-precision%29))
  (Transformation|SetActorLocation (Math|Vector|Lerp(Vector) (Variables|Default|GetCrystalLocation) (Variables|Default|GetBall_Location) Alpha) false false))

(fn CrystalLocation
  (bind _output_get (Variables|Default|SetStart_Location (Transformation|GetActorLocation)))
  (return _output_get))

(fn CrystalScale
  (params (Alpha :type Float%20%28single-precision%29))
  (Transformation|SetActorScale3D (Math|Vector|Lerp(Vector) (Variables|Default|GetCrystalScale) "0, 0, 0" Alpha)))

(fn CrystalLight
  (params (Alpha :type Float%20%28single-precision%29))
  (Rendering|Components|Light|SetIntensity (Variables|Default|GetPointLight) (Math|Float|Lerp (Variables|Default|GetCrystalLight) 0.0 Alpha)))

(fn SetVariables
  (Variables|Default|SetCrystalScale (Transformation|GetActorScale3D))
  (Variables|Default|SetCrystalLight (Variables|/Script/Engine.LightComponentBase|GetIntensity (Variables|Default|GetPointLight)))
  (Variables|Default|SetBall_Location (Transformation|GetActorLocation (Game|Player|GetPlayerPawn 0)))
  (Variables|Default|SetCrystalLocation (Transformation|GetActorLocation)))